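; BP_Test_Character is a test character Blueprint that exercises basic component, event and function mechanics.
; On BeginPlay it initializes its BPTestComponent.
; A custom TestEvent increments the RefCounter variable and prints the result.
; TestFunc adds a fixed offset to an input vector and returns its Z, along with an input string with a greeting appended.
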(event `self.ReceiveBeginPlay`
  (`/Game/Core/Blueprints/Test/BP_Test_Component.Initialize` (`self.BP_Test_Component`)))

(event `TestEvent`
  (bind _result (`/Engine/EditorBlueprintResources/StandardMacros.IncrementInt` (`self.RefCounter`))
    (:`  `
      (`KismetSystemLibrary.PrintString` (`KismetStringLibrary.Conv_IntToString` _result)))))

(fn `TestFunc`
  (params (NewParam :type "Float (double-precision)") (NewParam1 :type String))
  (returns (NewParam2 :type "Float (double-precision)") (NewParam3 :type String))
  (bind (_returnvalue_x _returnvalue_y _returnvalue_z) (`KismetMathLibrary.BreakVector` (+ (0.0 1.0 2.0) NewParam)))
  (return _returnvalue_z (`KismetStringLibrary.Concat_StrStr` NewParam1 "Hello")))

(fn `UserConstructionScript`)